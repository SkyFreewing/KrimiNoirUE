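; Background NPC character that assembles a modular body and wanders between three waypoint markers.
; The construction script applies upper and lower body meshes and materials, with the lower body following the main mesh's pose.
; When patrolling is enabled, BeginPlay stores marker locations as waypoints.
; Tick cycles through them, skipping markers with overlapping actors, and uses AI MoveTo, pausing randomly after each successful arrival.
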(event EventBeginPlay
  (if (Variables|Default|GetIsPatroling)
    (CallFunction|SetWaypoints)))

(event Collision|EventActorBeginOverlap
  (params (OtherActor :type Actor%20Object%20Reference)))

(event EventTick
  (params (DeltaSeconds :type Float%20%28single-precision%29))
  ;[1 1 1] ResetCounter
  (if (>= (Variables|Default|GetWaypointCounter) (Utilities|Array|Length (Variables|Default|GetWaypoints)))
    (Variables|Default|SetWaypointCounter 0))
  (if (not (Variables|Default|GetHasGoal))
    (if (== (Utilities|Array|Length (Collision|GetOverlappingActors (Utilities|Array|Get(acopy) (Variables|Default|GetWaypointMarker) (Variables|Default|GetWaypointCounter)) 0 :!class /Script/Engine.PrimitiveComponent)) 0)
      (Variables|Default|SetHasGoal true)
      (AI|AIMoveTo self (Utilities|Array|Get(acopy) (Variables|Default|GetWaypoints) (Variables|Default|GetWaypointCounter)) 0 5.0 false
        (:OnSuccess
          (Utilities|FlowControl|Delay (Math|Random|RandomFloatinRange 1.0 3e+01)))
        (:OnFail
          _))
      (Variables|Default|SetHasGoal false)
      (Math|Integer|IncrementInt (Variables|Default|GetWaypointCounter))
      (else
        (Math|Integer|IncrementInt (Variables|Default|GetWaypointCounter))))))

(fn ConstructionScript
  (Class|SkinnedMeshComponent|SetSkeletalMesh (Variables|Character|GetMesh) (Utilities|Array|Get(acopy) (Variables|Properties|GetUpperBodyMeshes)) true)
  (Class|SkinnedMeshComponent|SetSkeletalMesh (Variables|Default|GetLowerBody) (Utilities|Array|Get(acopy) (Variables|Properties|GetLowerBodyMeshes)) true)
  (for (_ _array_index) (Rendering|Material|GetMaterials (Variables|Default|GetLowerBody))
    (Rendering|Material|SetMaterial (Variables|Default|GetLowerBody) _array_index (Utilities|Array|Get(acopy) (Variables|Properties|GetLower%20Materials) _array_index)))
  (for (_ _array_index_2) (Rendering|Material|GetMaterials (Variables|Character|GetMesh))
    (Rendering|Material|SetMaterial (Variables|Character|GetMesh) _array_index_2 (Utilities|Array|Get(acopy) (Variables|Properties|GetUpper%20Materials) _array_index_2))
    (Class|SkinnedMeshComponent|SetMasterPoseComponent (Variables|Default|GetLowerBody) (Variables|Character|GetMesh) false)))

(fn SetWaypoints
  (bind _waypointmarker (Variables|Default|GetWaypointMarker))
  (Utilities|Array|SetArrayElem _waypointmarker 0 (Variables|Default|GetWaypoint1Marker))
  (Utilities|Array|Add _waypointmarker (Variables|Default|GetWaypoint2Marker))
  (Utilities|Array|Add _waypointmarker (Variables|Default|GetWaypoint3Marker))
  (for _array_element _waypointmarker
    (Utilities|Array|Add (Variables|Default|GetWaypoints) (Transformation|GetWorldLocation _array_element))))