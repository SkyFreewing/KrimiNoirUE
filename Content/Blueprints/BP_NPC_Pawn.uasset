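; NPC pawn Blueprint that builds a character from separate upper and lower body skeletal meshes, with no gameplay logic in its event graph.
; The construction script assigns both meshes from variables, then applies per-slot materials from the upper and lower material arrays.
; Inside the upper-body material loop, it sets UpperBody as LowerBody's master pose component, so both halves share one pose.
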(event EventBeginPlay)

(event Collision|EventActorBeginOverlap
  (params (OtherActor :type Actor%20Object%20Reference)))

(event EventTick
  (params (DeltaSeconds :type Float%20%28single-precision%29)))

(fn ConstructionScript
  (Class|SkinnedMeshComponent|SetSkeletalMesh (Variables|Default|GetUpperBody) (Variables|Mesh|GetUpperBodyNew) true)
  (Class|SkinnedMeshComponent|SetSkeletalMesh (Variables|Default|GetLowerBody) (Variables|Mesh|GetLowerBodyNew) true)
  (for (_ _array_index) (Rendering|Material|GetMaterials (Variables|Default|GetLowerBody))
    (Rendering|Material|SetMaterial (Variables|Default|GetLowerBody) _array_index (Utilities|Array|Get(acopy) (Variables|Materials|GetLower%20Materials) _array_index)))
  (for (_ _array_index_2) (Rendering|Material|GetMaterials (Variables|Default|GetUpperBody))
    (Rendering|Material|SetMaterial (Variables|Default|GetUpperBody) _array_index_2 (Utilities|Array|Get(acopy) (Variables|Materials|GetUpper%20Materials) _array_index_2))
    (Class|SkinnedMeshComponent|SetMasterPoseComponent (Variables|Default|GetLowerBody) (Variables|Default|GetUpperBody) false)))