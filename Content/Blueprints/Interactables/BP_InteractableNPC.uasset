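; Interactable NPC Blueprint that turns to face the player when interacted with.
; Interact calls the parent, captures the yaw difference toward player zero, then plays the Scaling timeline.
; Each timeline update steps yaw by that fixed difference times scale and delta time, preserving pitch and roll.
; SetupNPCBehaviour runs a behavior tree and sets the Idle blackboard flag, but nothing in this graph calls it.
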(event EventInteract
  (|CallParentFunction)
  (bind _rotation (CallFunction|GetPlayerLookatRot))
  (bind _scaling (Timeline|Scaling PlayFromStart)
    (:Update
      (CallFunction|RotatetoPlayer _scaling _rotation))))

(fn ConstructionScript
  (|CallParentFunction))

(fn RotatetoPlayer
  (params (Scale :type Float%20%28single-precision%29) (Rotation :type Rotator))
  (Transformation|SetActorRelativeRotation (Math|Rotator|MakeRotator (.roll Rotation) (.pitch Rotation) (- (.yaw (Transformation|GetActorRotation)) (* (Utilities|Time|GetWorldDeltaSeconds) (* (.yaw Rotation) Scale))))))

(fn SetupNPCBehaviour
  (bind _self self)
  (AI|RunBehaviorTree (AI|GetAIController _self) (Variables|Dialogue|GetBehaviorTree))
  (AI|Components|Blackboard|SetValueasBool (AI|GetBlackboard _self) (Utilities|Name|MakeLiteralName "Idle") true))

(fn GetPlayerLookatRot
  (bind _returnvalue (Game|GetPlayerCharacter 0))
  (bind _returnvalue_2 (Transformation|GetActorLocation))
  (bind _returnvalue_3 (Transformation|GetActorRotation))
  (bind _returnvalue_4 (Transformation|GetActorLocation _returnvalue))
  (bind _returnvalue_5 (Math|Rotator|FindLookatRotation _returnvalue_2 _returnvalue_4))
  (bind _returnvalue_6 (Math|Rotator|MakeRotator (.roll _returnvalue_3) (.pitch _returnvalue_3) (.yaw _returnvalue_5)))
  (return (Math|Rotator|MakeRotator (.roll _returnvalue_6) (.pitch _returnvalue_6) (- (.yaw (Transformation|GetActorRotation)) (.yaw _returnvalue_6)))))