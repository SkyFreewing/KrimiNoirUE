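; Dialogue component for the first-person character that plays an NPC's DataTable-driven conversation through a dialogue widget.
; It takes the NPC's table and progressed block, then scans rows for the matching Block and TextOrder, advancing the order per line once text display finishes.
; When no row matches, it clears state, closes the window and ends the owner's conversation.
; ShowProofSuccess jumps to a given block, skipping current text and advancing after a short delay.
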(event Custom|SkipCurrentDialogue
  (Default|SkipCurrentDialogue (Variables|Default|GetDialogueWindow)))

(event Custom|PostProofSkip
  (Utilities|FlowControl|Delay 0.1)
  (CallFunction|NextDialogue))

(fn GetNPCDialogueTable
  (params (NPC :type BP%20Interactable%20NPC%20Object%20Reference))
  (Utilities|IsValid NPC
    (:Is%20Valid
      (Variables|Default|SetCurrentDialogue (Variables|/Game/Blueprints/Interactables/BP_InteractableNPC.BP_InteractableNPC_C|GetDialogueTable NPC)))
    (:Is%20Not%20Valid
      (Development|PrintString "Could not receive valid NPC -- Dialogue Component"))))

(fn StartDialogue
  (params (Block :type Integer) (TextOrder :type Integer) (CharacterName :type Text))
  (bind _currentdialogue (Variables|Default|GetCurrentDialogue))
  (bind _outrownames (DataTable|GetDataTableRowNames _currentdialogue))
  (for _array_element _outrownames
    (bind _returnvalue (Utilities|GetDataTableRow _currentdialogue _array_element)
      (:then
        (if (and (== (.Block (Utilities|Struct|BreakS_DialogueText _returnvalue)) Block) (== (.TextOrder (Utilities|Struct|BreakS_DialogueText _returnvalue)) TextOrder))
          (Default|DisplayNewDialogue (Variables|Default|GetDialogueWindow) (.Text (Utilities|Struct|BreakS_DialogueText _returnvalue)) CharacterName)
          (Math|Integer|IncrementInt (Variables|Default|GetCurrentDialogueOrder)
            (:%20%20
              (return)))))))
  (CallFunction|EndCurrentDialogue))

(fn SetupDialoguetoPlay
  (params (NPC :type BP%20Interactable%20NPC%20Object%20Reference) (Character :type Text))
  (CallFunction|GetNPCDialogueTable NPC)
  (CallFunction|PickupCurrentDialogueStart (Variables|/Game/Blueprints/Interactables/BP_InteractableNPC.BP_InteractableNPC_C|GetProgressedBlock NPC))
  (CallFunction|NextDialogue Character))

(fn SetDialogueWidget
  (params (DialogueBox :type WBP%20Dialogue%20Box%20Object%20Reference))
  (Utilities|IsValid DialogueBox
    (:Is%20Valid
      (Variables|Default|SetDialogueWindow DialogueBox))
    (:Is%20Not%20Valid
      (Development|PrintString "Dialogue Box reference gotten is empty -- Dialogue Component"))))

(fn NextDialogue
  (params (Character%20Name :type Text))
  (if (Variables|/Game/Blueprints/DialogueSystem/WBP_DialogueBox.WBP_DialogueBox_C|GetTextDisplayDone (Variables|Default|GetDialogueWindow))
    (CallFunction|StartDialogue (Variables|Default|GetCurrentDialogueBlock) (Variables|Default|GetCurrentDialogueOrder) Character%20Name)))

(fn PickupCurrentDialogueStart
  (params (Block :type Integer) (Order :type Integer))
  (Variables|Default|SetCurrentDialogueBlock Block)
  (Variables|Default|SetCurrentDialogueOrder Order))

(fn EndCurrentDialogue
  (Variables|Default|SetCurrentDialogueOrder 0)
  (Variables|Default|SetCurrentDialogueBlock 0)
  (Variables|Default|SetCurrentDialogue 0)
  (Default|EndOfDialogue (Variables|Default|GetDialogueWindow))
  (bind _asfirst_person_character (Utilities|Casting|CastToFirstPersonCharacter (Components|GetOwner))
    (:then
      (Default|EndConversation _asfirst_person_character)
      (Development|PrintString "Dialogue ended!"))
    (:CastFailed
      (Development|PrintString "Trying to end dialogue -> Current owner is not FPCharacter -- Dialogue Component"))))

(fn ShowProofSuccess
  (params (Block :type Integer))
  (Variables|Default|SetCurrentDialogueOrder 0)
  (Variables|Default|SetCurrentDialogueBlock Block)
  (Default|SkipCurrentDialogue (Variables|Default|GetDialogueWindow))
  (CallFunction|PostProofSkip))