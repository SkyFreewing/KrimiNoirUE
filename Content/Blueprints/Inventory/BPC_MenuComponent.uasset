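; Inventory and menu component that tracks items and quest statements and drives the diary menu and dialogue box.
; Item changes update CurrentItems and fill or clear WBP_InventorySlot widgets in the menu's grid.
; New statements are filed under their matching quest in AllQuests, whose first statement creates a grid slot and later ones update its label.
; Menu and dialogue toggles switch cursor and input mode, restoring game-only input when neither is open.
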(event EventBeginPlay)

(event EventTick
  (params (DeltaSeconds :type Float%20%28single-precision%29)))

(fn AddItemtoInventory
  (params (NewItem :type S%20Inventory%20Item%20Structure))
  (Utilities|Array|AddUnique (Variables|Core|GetCurrentItems) NewItem)
  (Inventory|DisplayIteminInventory NewItem))

(fn RemoveItem
  (params (RemoveItem :type S%20Inventory%20Item%20Structure))
  (bind _returnvalue (Utilities|Array|RemoveItem (Variables|Core|GetCurrentItems) RemoveItem))
  (if _returnvalue
    (Inventory|RemoveItemfromInventory RemoveItem)
    (else
      (Development|PrintString "Inventory collection did not contain item to be removed -- Inventory Component"))))

(fn GetItembyIndex
  (params (Index :type Integer))
  (LocalVariables|SetLocalIndex Index)
  (if (Utilities|Array|IsValidIndex (Variables|Core|GetCurrentItems) (LocalVariables|GetLocalIndex))
    (return (Utilities|Array|Get(acopy) (Variables|Core|GetCurrentItems) (LocalVariables|GetLocalIndex)))
    (else
      (Development|PrintString "Tried to get Item with invalid Index from CurrentItems"))))

(fn CheckInventoryforItem
  (params (ItemNameToCheck :type String))
  (if (Utilities|Enum|NotEqual(Enum) ItemNameToCheck "")
    (LocalVariables|SetLocalNameToCheck ItemNameToCheck)
    (for _array_element (Variables|Core|GetCurrentItems)
      (if (Utilities|Enum|Equal(Enum) (.Name (Utilities|Struct|BreakS_InventoryItem _array_element)) (LocalVariables|GetLocalNameToCheck))
        (return true)))
    (return false)
    (else
      (Development|PrintString "Tried to execute inventory check with empty name"))))

(fn PrintInventory
  (Development|PrintString "Current Inventory:")
  (for (_array_element _array_index) (Variables|Core|GetCurrentItems)
    (Development|PrintString (Utilities|String|ToString(Integer) _array_index))
    (Development|PrintString (.name _array_element))))

(fn SetMenuWidgets
  (params (MenuWidget :type WBP%20Player%20Menu%20Screen%20Object%20Reference))
  (Utilities|IsValid MenuWidget
    (:Is%20Valid
      (bind _output_get (Variables|Core|SetMenuWidget MenuWidget))
      (bind _output_get_2 (Variables|Core|SetDialogueWidget (Variables|/Game/Blueprints/Inventory/WBP_PlayerMenuScreen.WBP_PlayerMenuScreen_C|GetWBP_DialogueBox _output_get)))
      (Widget|SetVisibility (Variables|/Game/Blueprints/Inventory/WBP_PlayerMenuScreen.WBP_PlayerMenuScreen_C|GetDiaryBorder _output_get) "Hidden")
      (Widget|SetVisibility _output_get_2 "Hidden"))
    (:Is%20Not%20Valid
      (Development|PrintString "Menu reference gotten is empty -- Inventory Component"))))

(fn DisplayIteminInventory
  (params (Item :type S%20Inventory%20Item%20Structure))
  (LocalVariables|SetLocalItemStruct Item)
  (for _array_element (Class|PanelWidget|GetAllChildren (Variables|/Game/Blueprints/Inventory/WBP_PlayerMenuScreen.WBP_PlayerMenuScreen_C|GetInventoryGrid (Variables|Core|GetMenuWidget)))
    (bind _aswbp_inventory_slot (Utilities|Casting|CastToWBP_InventorySlot _array_element)
      (:then
        (if (not (Variables|/Game/Blueprints/Inventory/WBP_InventorySlot.WBP_InventorySlot_C|GetHasItem _aswbp_inventory_slot))
          (Default|DisplayItem _aswbp_inventory_slot (LocalVariables|GetLocalItemStruct) true)
          (Development|PrintString "Added: ")
          (Development|PrintString (.label (LocalVariables|GetLocalItemStruct)))
          (return)))
      (:CastFailed
        (Development|PrintString "Casted Widget was no inventory slot when trying to display -- Inventory Component"))))
  (Development|PrintString "Inventory Overflow"))

(fn RemoveItemfromInventory
  (params (Item :type S%20Inventory%20Item%20Structure))
  (LocalVariables|SetLocalItem Item)
  (for _array_element (Class|PanelWidget|GetAllChildren (Variables|/Game/Blueprints/Inventory/WBP_PlayerMenuScreen.WBP_PlayerMenuScreen_C|GetInventoryGrid (Variables|Core|GetMenuWidget)))
    (bind _aswbp_inventory_slot (Utilities|Casting|CastToWBP_InventorySlot _array_element)
      (:then
        (if (and (Variables|/Game/Blueprints/Inventory/WBP_InventorySlot.WBP_InventorySlot_C|GetHasItem _aswbp_inventory_slot) (Utilities|Enum|Equal(Enum) (Variables|/Game/Blueprints/Inventory/WBP_InventorySlot.WBP_InventorySlot_C|GetItemName _aswbp_inventory_slot) (.name (LocalVariables|GetLocalItem))))
          (Default|DisplayItem _aswbp_inventory_slot (LocalVariables|GetLocalItem) false)
          (return)))
      (:CastFailed
        (Development|PrintString "Casted Widget was no inventory slot when trying to remove -- Inventory Component"))))
  (Development|PrintString "Inventory didn't contain item name"))

(fn ToggleMenu
  (params (Toggle :type Boolean))
  (bind _returnvalue (Game|GetPlayerController 0))
  (bind _menuwidget (Variables|Core|GetMenuWidget))
  (bind _diaryborder (Variables|/Game/Blueprints/Inventory/WBP_PlayerMenuScreen.WBP_PlayerMenuScreen_C|GetDiaryBorder _menuwidget))
  (if Toggle
    (Widget|SetVisibility _diaryborder "Visible")
    (Variables|/Script/Engine.PlayerController|SetbShowMouseCursor _returnvalue true)
    (Input|SetInputModeGameandUI _returnvalue (Variables|Core|GetMenuWidget) "LockAlways" true)
    (else
      (Widget|SetVisibility _diaryborder "Hidden")
      (Default|ResetMenu (Variables|Core|GetMenuWidget))
      (if (not (Variables|Status|GetDialogueOpen))
        (Variables|/Script/Engine.PlayerController|SetbShowMouseCursor _returnvalue false)
        (Input|SetInputModeGameOnly _returnvalue)))))

(fn ToggleDialogueBox
  (params (Toggle :type Boolean))
  (bind _returnvalue (Game|GetPlayerController 0))
  (bind _menuwidget (Variables|Core|GetMenuWidget))
  (bind _wbp_dialoguebox (Variables|/Game/Blueprints/Inventory/WBP_PlayerMenuScreen.WBP_PlayerMenuScreen_C|GetWBP_DialogueBox _menuwidget))
  (if Toggle
    (Widget|SetVisibility _wbp_dialoguebox "Visible")
    (Variables|/Script/Engine.PlayerController|SetbShowMouseCursor _returnvalue true)
    (Input|SetInputModeGameandUI _returnvalue (Variables|Core|GetMenuWidget) "LockAlways" true)
    (else
      (Widget|SetVisibility _wbp_dialoguebox "Hidden")
      (if (not (Variables|Status|GetMenuOpen))
        (Variables|/Script/Engine.PlayerController|SetbShowMouseCursor _returnvalue false)
        (Input|SetInputModeGameOnly _returnvalue)))))

(fn AddNewStatement
  (params (NewStatement :type S%20Statement%20Structure))
  (Utilities|Array|AddUnique (Variables|Core|GetCurrentStatements) NewStatement))

(fn CheckStatementsforName
  (params (ItemNameToCheck :type String))
  (if (Utilities|Enum|NotEqual(Enum) ItemNameToCheck "")
    (LocalVariables|SetLocalNameToCheck ItemNameToCheck)
    (for _array_element (Variables|Core|GetAllQuests)
      (for _array_element_2 (.statements _array_element)
        (if (Utilities|Enum|Equal(Enum) "" (LocalVariables|GetLocalNameToCheck))
          (return true))))
    (return false)
    (else
      (Development|PrintString "Tried to execute inventory check with empty name"))))

(fn UpdateStatements
  (params (Statement :type S%20Statement%20Structure))
  (bind (_quest _label) (Utilities|Struct|BreakS_Statement Statement))
  (bind _allquests (Variables|Core|GetAllQuests))
  (for (_array_element _array_index) (Variables|Core|GetAllQuests)
    (bind _output_get (LocalVariables|SetLocalArray (.statements _array_element)))
    (if (Utilities|Enum|Equal(Enum) (.label _array_element) _quest)
      (bind _returnvalue (Utilities|Array|AddUnique _output_get _label))
      (if (!= _returnvalue -1)
        (Statements|AddNewStatement Statement)
        (Utilities|Array|SetArrayElem _allquests _array_index (Utilities|Struct|MakeS_Quest (.label (Utilities|Array|Get(acopy) _allquests _array_index)) (.fullname (Utilities|Array|Get(acopy) _allquests _array_index)) (.icon (Utilities|Array|Get(acopy) _allquests _array_index)) _output_get))
        (if (== (Utilities|Array|Length _output_get) 1)
          (Inventory|DisplayIteminInventory (Utilities|Struct|MakeS_InventoryItem (.label _array_element) _label (.icon _array_element) 0 0))
          (else
            (for _array_element_2 (Class|PanelWidget|GetAllChildren (Variables|/Game/Blueprints/Inventory/WBP_PlayerMenuScreen.WBP_PlayerMenuScreen_C|GetInventoryGrid (Variables|Core|GetMenuWidget)))
              (bind _aswbp_inventory_slot (Utilities|Casting|CastToWBP_InventorySlot _array_element_2))
              (if (Utilities|Enum|Equal(Enum) (.label _array_element) (Variables|/Game/Blueprints/Inventory/WBP_InventorySlot.WBP_InventorySlot_C|GetItemName _aswbp_inventory_slot))
                (Default|UpdateLabel _aswbp_inventory_slot _label)))))))))

(fn CheckQuestorItem
  (params (Name :type String))
  (for _array_element (Variables|Core|GetAllQuests)
    (if (Utilities|Enum|Equal(Enum) (.label _array_element) Name)
      (bind _statements (Statements|GetAllStatementsOfQuest (.label _array_element)))
      (return true _statements (.fullname _array_element))))
  (return false 0 Name))

(fn GetStatement
  (params (Label :type String))
  (for _array_element (Variables|Core|GetCurrentStatements)
    (if (Utilities|Enum|Equal(Enum) (.Label (Utilities|Struct|BreakS_Statement _array_element)) Label)
      (return _array_element))))

(fn GetAllStatementsOfQuest
  (params (Quest :type String))
  (bind _statementstoreturn (LocalVariables|GetStatementsToReturn))
  (for _array_element (Variables|Core|GetAllQuests)
    (if (Utilities|Enum|Equal(Enum) Quest (.label _array_element))
      (for _array_element_2 (.statements _array_element)
        (for _array_element_3 (Variables|Core|GetCurrentStatements)
          (if (Utilities|Enum|Equal(Enum) _array_element_2 (.Label (Utilities|Struct|BreakS_Statement _array_element_3)))
            (Utilities|Array|Add _statementstoreturn _array_element_3))))))
  (return _statementstoreturn))