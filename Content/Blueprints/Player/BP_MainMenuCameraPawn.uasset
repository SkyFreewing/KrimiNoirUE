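; Main menu camera pawn that player 0 possesses on BeginPlay to present the main menu.
; It creates WBP_MainMenu, shows the cursor in Game and UI input mode, and passes itself to the widget via GetCameraPawn.
; BeginTheGame hides the menu, restores game-only input without a cursor, and hands possession to the referenced PlayerCharacter.
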(event EventBeginPlay
  (Pawn|Possess (Game|GetPlayerController 0) self)
  (CallFunction|SetupMainMenuWidget))

(fn ConstructionScript)

(fn SetupMainMenuWidget
  (bind _returnvalue (Game|GetPlayerController 0))
  (bind _returnvalue_2 (UserInterface|CreateWidget "/Game/Blueprints/Inventory/WBP_MainMenu.WBP_MainMenu_C" _returnvalue))
  (Input|SetInputModeGameandUI _returnvalue _returnvalue_2 "DoNotLock" true)
  (UserInterface|Viewport|AddtoViewport _returnvalue_2 0)
  (Variables|/Script/Engine.PlayerController|SetbShowMouseCursor _returnvalue true)
  (bind _output_get (Variables|Default|SetMainMenuWidget _returnvalue_2))
  (Default|GetCameraPawn _output_get self))

(fn BegintheGame
  (bind _returnvalue (Game|GetPlayerController 0))
  (Widget|SetVisibility (Variables|Default|GetMainMenuWidget) "Hidden")
  (Input|SetInputModeGameOnly _returnvalue)
  (Variables|/Script/Engine.PlayerController|SetbShowMouseCursor _returnvalue false)
  (Pawn|Possess _returnvalue (Variables|Default|GetPlayerCharacter)))