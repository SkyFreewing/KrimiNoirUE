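; Spline-driven street prop that builds colliding spline mesh segments along its spline in the Construction Script.
; The center loop lays MeshLength-long segments, skipping the first index, with tangents clamped to that length for bending along the curve.
; FirstPart and LastPart add short end pieces at hand-tuned offsets, the first at fixed distances and the last relative to the final whole segment.
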(fn ConstructionScript
  (|FirstPart)
  (|LoopCenterParts)
  (|LastPart))