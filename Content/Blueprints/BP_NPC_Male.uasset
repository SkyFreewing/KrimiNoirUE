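; BP_NPC_Male is a modular male NPC whose appearance is assembled from separate upper and lower body skeletal meshes.
; The construction script applies the mesh and material variables to each half, overriding the first material slot.
; The lower body uses the upper body as its master pose component, so both halves share one pose.
; The event graph holds only disabled placeholder events, so the Blueprint adds no runtime logic.
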(event EventBeginPlay)

(event Collision|EventActorBeginOverlap
  (params (OtherActor :type Actor%20Object%20Reference)))

(event EventTick
  (params (DeltaSeconds :type Float%20%28single-precision%29)))

(fn ConstructionScript
  (Class|SkinnedMeshComponent|SetSkeletalMesh (Variables|Default|GetUpperBody) (Variables|Mesh|GetUpperBodyNew) true)
  (Class|SkinnedMeshComponent|SetSkeletalMesh (Variables|Default|GetLowerBody) (Variables|Mesh|GetLowerBodyNew) true)
  (Rendering|Material|SetMaterial (Variables|Default|GetUpperBody) 0 (Variables|Materials|GetUpperBodyMat))
  (Rendering|Material|SetMaterial (Variables|Default|GetLowerBody) 0 (Variables|Materials|GetLowerBodyMat))
  (Class|SkinnedMeshComponent|SetMasterPoseComponent (Variables|Default|GetLowerBody) (Variables|Default|GetUpperBody) false))