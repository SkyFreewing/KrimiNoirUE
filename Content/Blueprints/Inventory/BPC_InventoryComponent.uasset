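; Inventory component that keeps an array of item structs and mirrors it into the slot widgets of a menu's inventory grid.
; Adding stores the item uniquely and fills the first empty slot; removing clears the first occupied slot with a matching name.
; Helpers fetch by index, print the contents and receive the menu widget reference, with failures reported through PrintString.
; The by-name check compares no names, returning the first item whenever any exists.
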(event EventBeginPlay)

(event EventTick
  (params (DeltaSeconds :type Float%20%28single-precision%29)))

(fn AddItemtoInventory
  (params (NewItem :type S%20Inventory%20Item%20Structure))
  (Utilities|Array|AddUnique (Variables|Core|GetCurrentItems) NewItem)
  (CallFunction|DisplayIteminInventory NewItem))

(fn RemoveItem
  (params (RemoveItem :type S%20Inventory%20Item%20Structure))
  (bind _returnvalue (Utilities|Array|RemoveItem (Variables|Core|GetCurrentItems) RemoveItem))
  (if _returnvalue
    (CallFunction|RemoveItemfromInventory RemoveItem)
    (else
      (Development|PrintString "Inventory collection did not contain item to be removed -- Inventory Component"))))

(fn GetItembyIndex
  (params (Index :type Integer))
  (LocalVariables|SetLocalIndex Index)
  (if (Utilities|Array|IsValidIndex (Variables|Core|GetCurrentItems) (LocalVariables|GetLocalIndex))
    (return (Utilities|Array|Get(acopy) (Variables|Core|GetCurrentItems) (LocalVariables|GetLocalIndex)))
    (else
      (Development|PrintString "Tried to get Item with invalid Index from CurrentItems"))))

(fn CheckInventoryforItem
  (params (ItemNameToCheck :type String))
  (if (Utilities|Enum|NotEqual(Enum) ItemNameToCheck "")
    (LocalVariables|SetLocalNameToCheck ItemNameToCheck)
    (for (_array_element _array_index) (Variables|Core|GetCurrentItems)
      (if true
        (return true _array_element _array_index)))
    (return false "" 0)
    (else
      (Development|PrintString "Tried to execute inventory check with empty name"))))

(fn PrintInventory
  (Development|PrintString "Current Inventory:")
  (for (_array_element _array_index) (Variables|Core|GetCurrentItems)
    (Development|PrintString (Utilities|String|ToString(Integer) _array_index))
    (Development|PrintString (.name _array_element))))

(fn SetMenuWidget
  (params (MenuWidget :type WBP%20Player%20Menu%20Screen%20Object%20Reference))
  (Utilities|IsValid MenuWidget
    (:Is%20Valid
      (Variables|Core|SetMenuWidget MenuWidget))
    (:Is%20Not%20Valid
      (Development|PrintString "Menu reference gotten is empty -- Inventory Component"))))

(fn DisplayIteminInventory
  (params (Item :type S%20Inventory%20Item%20Structure))
  (LocalVariables|SetLocalItemStruct Item)
  (for _array_element (Class|PanelWidget|GetAllChildren (Variables|/Game/Blueprints/Inventory/WBP_PlayerMenuScreen.WBP_PlayerMenuScreen_C|GetInventoryGrid (Variables|Core|GetMenuWidget)))
    (bind _aswbp_inventory_slot (Utilities|Casting|CastToWBP_InventorySlot _array_element)
      (:then
        (if (not (Variables|/Game/Blueprints/Inventory/WBP_InventorySlot.WBP_InventorySlot_C|GetHasItem _aswbp_inventory_slot))
          (Default|DisplayItem _aswbp_inventory_slot (LocalVariables|GetLocalItemStruct) true)
          (Development|PrintString "Added: ")
          (Development|PrintString (.name (LocalVariables|GetLocalItemStruct)))
          (return)))
      (:CastFailed
        (Development|PrintString "Casted Widget was no inventory slot when trying to display -- Inventory Component"))))
  (Development|PrintString "Inventory Overflow"))

(fn RemoveItemfromInventory
  (params (Item :type S%20Inventory%20Item%20Structure))
  (LocalVariables|SetLocalItem Item)
  (for _array_element (Class|PanelWidget|GetAllChildren (Variables|/Game/Blueprints/Inventory/WBP_PlayerMenuScreen.WBP_PlayerMenuScreen_C|GetInventoryGrid (Variables|Core|GetMenuWidget)))
    (bind _aswbp_inventory_slot (Utilities|Casting|CastToWBP_InventorySlot _array_element)
      (:then
        (if (and (Variables|/Game/Blueprints/Inventory/WBP_InventorySlot.WBP_InventorySlot_C|GetHasItem _aswbp_inventory_slot) (Utilities|Enum|Equal(Enum) (Variables|/Game/Blueprints/Inventory/WBP_InventorySlot.WBP_InventorySlot_C|GetItemName _aswbp_inventory_slot) (.name (LocalVariables|GetLocalItem))))
          (Default|DisplayItem _aswbp_inventory_slot (LocalVariables|GetLocalItem) false)
          (return)))
      (:CastFailed
        (Development|PrintString "Casted Widget was no inventory slot when trying to remove -- Inventory Component"))))
  (Development|PrintString "Inventory didn't contain item name"))