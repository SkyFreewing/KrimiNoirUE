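; Base Blueprint for interactable objects, with a mesh, a sphere trigger radius and a widget component for the interaction prompt.
; The construction script applies the configurable mesh, scale, offsets and trigger range, and makes the widget visible.
; BeginPlay passes InteractionText to the WBP_InteractHighlight widget, printing an error if the cast fails.
; Interact is an empty event, and SetDisplayWidget toggles prompt visibility; no overlap handling is defined here.
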(event Custom|Interact)

(event EventBeginPlay
  (CallFunction|SetupUIText))

(fn ConstructionScript
  (CallFunction|Setup))

(fn SetDisplayWidget
  (params (New%20Visibility :type Boolean))
  (Rendering|SetVisibility (Variables|Default|GetDisplayWidget) New%20Visibility false))

(fn Setup
  (Components|StaticMesh|SetStaticMesh (Variables|Default|GetStaticMesh) (Variables|Properties|GetMesh))
  (Transformation|SetRelativeScale3D (Variables|Default|GetStaticMesh) (Variables|Properties|GetMeshScale))
  (Transformation|SetRelativeLocation (Variables|Default|GetStaticMesh) (Variables|Properties|GetMeshOffset) false false)
  (Components|Sphere|SetSphereRadius (Variables|Default|GetTriggerRadius) (Variables|Properties|GetTriggerRange) true)
  (Rendering|SetVisibility (Variables|Default|GetDisplayWidget) true false)
  (Transformation|SetRelativeLocation (Variables|Default|GetDisplayWidget) (Variables|Properties|GetWidgetOffset) false false))

(fn SetupUIText
  (bind _aswbp_interact_highlight (Utilities|Casting|CastToWBP_InteractHighlight (UserInterface|GetUserWidgetObject (Variables|Default|GetDisplayWidget)))
    (:then
      (Variables|/Game/Blueprints/Interactables/WBP_InteractHighlight.WBP_InteractHighlight_C|SetInteractionText _aswbp_interact_highlight (Variables|Properties|GetInteractionText)))
    (:CastFailed
      (Development|PrintString "Display Widget could not be cast"))))